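; Base Blueprint for town buildings that shows a talk widget nearby and opens a building menu on interaction.
; BeginPlay passes the owner name, picture and chat list to TalkUI, which is shown or removed as BP_FieldChar enters or leaves overlap.
; Interact removes TalkUI, adds a focusable BuildingUI widget, swaps Enhanced Input from the field to the menu mapping context, and shows the mouse cursor.
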(event `self.ReceiveBeginPlay`
  (bind _talkui (`self.TalkUI`))
  (set `/Game/Game/UI/Dialogue/WBP_Dialogue.OwnerName` (`self.OwnerName`) _talkui)
  (set `/Game/Game/UI/Dialogue/WBP_Dialogue.OwnerPic` (`self.BuildingPic`) _talkui)
  (set `/Game/Game/UI/Dialogue/WBP_Dialogue.OwnerTalkList` (`self.BuildingChatList`) _talkui))

(event `self.ReceiveActorBeginOverlap`
  (params (OtherActor :type "Actor Object Reference"))
  (cast `/Game/Game/Blueprints/Pawns/BP_FieldChar` OtherActor)
  (`UserWidget.AddToViewport` (`self.TalkUI`) 0))

(event `self.ReceiveActorEndOverlap`
  (params (OtherActor :type "Actor Object Reference"))
  (cast `/Game/Game/Blueprints/Pawns/BP_FieldChar` OtherActor)
  (`Widget.RemoveFromParent` (`self.TalkUI`)))

(event `self.Interact`
  (bind _returnvalue (`GameplayStatics.GetPlayerController` 0))
  (bind _buildingu (`self.BuildingU`))
  (bind _returnvalue_2 (pcsubsystem `EnhancedInputLocalPlayerSubsystem` _returnvalue))
  (`Widget.RemoveFromParent` (`self.TalkUI`))
  (`|CreateWidget` (`self.BuildingUI`))
  (set `UserWidget.bIsFocusable` true _buildingu)
  (`UserWidget.AddToViewport` _buildingu 0)
  (`/Engine/EditorBlueprintResources/StandardMacros.IsValid` _returnvalue_2
    (:`Is Valid`
      (`EnhancedInputSubsystemInterface.RemoveMappingContext` _returnvalue_2 "/Game/Game/Inputs/IMC/IMC-Field.IMC-Field" (struct))
      (`EnhancedInputSubsystemInterface.AddMappingContext` _returnvalue_2 "/Game/Game/Inputs/IMC/IMC-Menu.IMC-Menu" 0 (struct))
      (set `PlayerController.bShowMouseCursor` true _returnvalue))))

(fn `UserConstructionScript`
  (`parent.UserConstructionScript`))