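; BP_BuidlingGeneral is the town's General building actor, which supplies the content for its WBP_General UI widget.
; On BeginPlay it runs the parent logic, casts BuildingUI to WBP_General, then copies in its items, owner picture and owner dialogue list.
; It adds no other active logic; the construction script only calls the parent and the overlap event is disabled.
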(event `self.ReceiveBeginPlay`
  (`parent.ReceiveBeginPlay`)
  (bind _aswbp_general (cast `/Game/Game/UI/Town/WBP_General` (`self.BuildingUI`)))
  (set `/Game/Game/UI/Town/WBP_General.Items` (`self.Items`) _aswbp_general)
  (set `/Game/Game/UI/Town/WBP_General.OwnerPic` (`self.BuildingPic`) _aswbp_general)
  (set `/Game/Game/UI/Town/WBP_General.OwnerDialogueList` (`self.GeneralDialogueList`) _aswbp_general))

(fn `UserConstructionScript`
  (`parent.UserConstructionScript`))