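; Base turn-based battle actor for party members and enemies, holding stats, targets and the skill to cast.
; Hovering shows its target widget; clicking makes it a target and casts the current player battler's skill.
; CastSkill checks costs, runs attack, defend or flee, then advances WBP_Battle's turn.
; TakeDamage clamps the stat, updates BP_BattleManager's alive/dead lists and checks win/lose; guarding does not yet reduce damage.
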(event `self.CapsuleComponent.OnBeginCursorOver`
  (params (TouchedComponent :type "PrimitiveComponent Object Reference"))
  (`self.MouseOver` true))

(event `self.CapsuleComponent.OnEndCursorOver`
  (params (TouchedComponent :type "PrimitiveComponent Object Reference"))
  (`self.MouseOver` false))

(event `self.CapsuleComponent.OnReleased`
  (params (TouchedComponent :type "PrimitiveComponent Object Reference") (ButtonReleased :type "Key Structure"))
  (`self.MouseClick`))

(event `self.ReceiveBeginPlay`
  (bind _aswbp_target_bar (cast `/Game/Game/UI/Battle/WBP_TargetBar` (`WidgetComponent.GetWidget` (`self.TargetUI`))))
  (set `/Game/Game/UI/Battle/WBP_TargetBar.AssignedChar` self _aswbp_target_bar))

(event `MouseOver`
  (params (Over :type Boolean))
  (`SceneComponent.SetVisibility` (`self.TargetUI`) Over false))

(event `MouseClick`
  (`self.ClickTargets`))

(fn `AddRemoveChar`
  (if (> (`BlueprintMapLibrary.Map_Find` (`.CurStats_24_6BED9ABA453EF44636EAB4B76C167FBD` (break `/Game/Game/Structs/S_Stats` (`self.Stats`))) "NewEnumerator0") 0.0)
    (bind _returnvalue (`GameplayStatics.GetActorOfClass` "/Game/Game/Blueprints/Pawns/BP_BattleManager.BP_BattleManager_C"))
    (bind _alivebattlechars (`/Game/Game/Blueprints/Pawns/BP_BattleManager.AliveBattleChars` _returnvalue))
    (if (not (`KismetArrayLibrary.Array_Contains` _alivebattlechars self))
      (`KismetArrayLibrary.Array_Add` _alivebattlechars self)
      (`KismetArrayLibrary.Array_RemoveItem` (`/Game/Game/Blueprints/Pawns/BP_BattleManager.DeadBattleChars` _returnvalue) self)
      (bind _asbp_battler_p (cast `/Game/Game/Blueprints/Pawns/BP_BattlerP` self)
        (:`then`
          (`KismetArrayLibrary.Array_Add` (`/Game/Game/Blueprints/Pawns/BP_BattleManager.AliveParty` _returnvalue) _asbp_battler_p))
        (:`CastFailed`
          (bind _asbp_battler_e (cast `/Game/Game/Blueprints/Enemies/BP_BattlerE` self))
          (`KismetArrayLibrary.Array_Add` (`/Game/Game/Blueprints/Pawns/BP_BattleManager.EnemyParty` _returnvalue) _asbp_battler_e))))
    (else
      (bind _returnvalue_2 (`GameplayStatics.GetActorOfClass` "/Game/Game/Blueprints/Pawns/BP_BattleManager.BP_BattleManager_C"))
      (bind _deadbattlechars (`/Game/Game/Blueprints/Pawns/BP_BattleManager.DeadBattleChars` _returnvalue_2))
      (if (not (`KismetArrayLibrary.Array_Contains` _deadbattlechars self))
        (`KismetArrayLibrary.Array_RemoveItem` (`/Game/Game/Blueprints/Pawns/BP_BattleManager.AliveBattleChars` _returnvalue_2) self)
        (`KismetArrayLibrary.Array_Add` _deadbattlechars self)
        (bind _asbp_battler_p_2 (cast `/Game/Game/Blueprints/Pawns/BP_BattlerP` self)
          (:`then`
            (`KismetArrayLibrary.Array_RemoveItem` (`/Game/Game/Blueprints/Pawns/BP_BattleManager.AliveParty` _returnvalue_2) _asbp_battler_p_2)
            (bind _foundwidgets (`WidgetBlueprintLibrary.GetAllWidgetsOfClass` "/Game/Game/UI/Battle/WBP_Battle.WBP_Battle_C"))
            (for _array_element _foundwidgets
              (`KismetArrayLibrary.Array_RemoveItem` (`/Game/Game/UI/Battle/WBP_Battle.TurnOrder` _array_element) self)))
          (:`CastFailed`
            (bind _asbp_battler_e_2 (cast `/Game/Game/Blueprints/Enemies/BP_BattlerE` self))
            (`KismetArrayLibrary.Array_RemoveItem` (`/Game/Game/Blueprints/Pawns/BP_BattleManager.EnemyParty` _returnvalue_2) _asbp_battler_e_2)
            (bind _foundwidgets_2 (`WidgetBlueprintLibrary.GetAllWidgetsOfClass` "/Game/Game/UI/Battle/WBP_Battle.WBP_Battle_C"))
            (for _array_element_2 _foundwidgets_2
              (`KismetArrayLibrary.Array_RemoveItem` (`/Game/Game/UI/Battle/WBP_Battle.TurnOrder` _array_element_2) self)
              (`self.K2_DestroyActor`))))))))

(fn `CastSkill`
  (params (SkillToCast :type "/Game/Game/Structs/Skills/S_Skill Structure"))
  (bind (_skilltype _secondaryaction _name _displayname _description _costmp _costhp _targettype _wantdead_ _power) (break `/Game/Game/Structs/Skills/S_Skill` SkillToCast))
  (bind (_name_2 _displayname_2 _lvl _icon _curstats) (break `/Game/Game/Structs/S_Stats` (`self.Stats`)))
  (bind _output_get (set `self.Done` (and (> (- (`BlueprintMapLibrary.Map_Find` _curstats "NewEnumerator1") _costmp) 0.0) (> (- (`BlueprintMapLibrary.Map_Find` _curstats "NewEnumerator0") _costhp) 0.0))))
  (if _output_get
    (switch `/Game/Game/Enums/E_SkillType` _skilltype
      (:`NewEnumerator0`
        (for _array_element (`self.Targets`)
          (`self.TakeDamage` _array_element (+ _power (`BlueprintMapLibrary.Map_Find` _curstats "NewEnumerator2")))
          (bind _foundwidgets (`WidgetBlueprintLibrary.GetAllWidgetsOfClass` "/Game/Game/UI/Battle/WBP_Battle.WBP_Battle_C" :!label _label))
          (`/Game/Game/UI/Battle/WBP_Battle.NewTurn` (`|GetArrayItem` _foundwidgets))))
      (:`NewEnumerator1`
        (set `self.Guarding` true)
        (goto _label))
      (:`NewEnumerator3`
        (if (< (`KismetMathLibrary.RandomInteger` 10) 5)
          (bind _asbp_game_instance (cast `/Game/Game/Blueprints/Basics/BP_GameInstance` (`GameplayStatics.GetGameInstance`)))
          (`GameplayStatics.OpenLevel` (`KismetStringLibrary.Conv_StringToName` (`.MapName_37_490558294894E216AB5D20BDAC0F04C5` (break `/Game/Game/Structs/S_SaveData` (`/Game/Game/Blueprints/Basics/BP_GameInstance.CurrentSaveData` _asbp_game_instance)))))
          (goto _label))))))

(fn `ClickTargets`
  (bind _player (`self.Player`))
  (bind _foundwidgets (`WidgetBlueprintLibrary.GetAllWidgetsOfClass` "/Game/Game/UI/Battle/WBP_Battle.WBP_Battle_C"))
  (for _array_element _foundwidgets
    (bind _asbp_battler_p (cast `/Game/Game/Blueprints/Pawns/BP_BattlerP` (`/Game/Game/UI/Battle/WBP_Battle.CurBattler` _array_element)))
    (bind _skilltocast (`/Game/Game/Blueprints/Battle/BP_Battler.SkillToCast` _asbp_battler_p))
    (switch `/Game/Game/Enums/E_SkillTarget` (`.TargetType_23_1C7801E040A11E825F5DBB87FFFABFD2` (break `/Game/Game/Structs/Skills/S_Skill` _skilltocast))
      (:`NewEnumerator1`
        (if _player
          (bind _targets (`/Game/Game/Blueprints/Battle/BP_Battler.Targets` _asbp_battler_p))
          (`KismetArrayLibrary.Array_Add` _targets self)
          (`self.CastSkill` _asbp_battler_p _skilltocast :!label _label)))
      (:`NewEnumerator2`
        (if (not _player)
          (`KismetArrayLibrary.Array_Add` _targets self)
          (goto _label)))
      (:`NewEnumerator3`
        (if _player
          (bind _returnvalue (`GameplayStatics.GetActorOfClass` "/Game/Game/Blueprints/Pawns/BP_BattleManager.BP_BattleManager_C"))
          (`KismetArrayLibrary.Array_Append` _targets (`/Game/Game/Blueprints/Pawns/BP_BattleManager.AliveParty` _returnvalue))
          (goto _label)))
      (:`NewEnumerator6`
        (if (not _player)
          (bind _returnvalue_2 (`GameplayStatics.GetActorOfClass` "/Game/Game/Blueprints/Pawns/BP_BattleManager.BP_BattleManager_C"))
          (`KismetArrayLibrary.Array_Append` _targets (`/Game/Game/Blueprints/Pawns/BP_BattleManager.EnemyParty` _returnvalue_2))
          (goto _label)))
      (:`NewEnumerator4`
        (bind _returnvalue_3 (`GameplayStatics.GetActorOfClass` "/Game/Game/Blueprints/Pawns/BP_BattleManager.BP_BattleManager_C"))
        (`KismetArrayLibrary.Array_Append` _targets (`/Game/Game/Blueprints/Pawns/BP_BattleManager.AliveBattleChars` _returnvalue_3))
        (goto _label))
      (:`NewEnumerator5`
        (`KismetArrayLibrary.Array_Add` _targets self)
        (goto _label)))))

(fn `SetTargets`
  (params (Skill :type "/Game/Game/Structs/Skills/S_Skill Structure"))
  (bind _targets (`self.Targets`))
  (bind _player (`self.Player`))
  (bind _returnvalue (`GameplayStatics.GetActorOfClass` "/Game/Game/Blueprints/Pawns/BP_BattleManager.BP_BattleManager_C"))
  (switch `/Game/Game/Enums/E_SkillTarget` (`.TargetType_23_1C7801E040A11E825F5DBB87FFFABFD2` (break `/Game/Game/Structs/Skills/S_Skill` Skill))
    (:`NewEnumerator1`
      (if _player
        (bind _aliveparty (`/Game/Game/Blueprints/Pawns/BP_BattleManager.AliveParty` _returnvalue))
        (for (_array_element _array_index) _aliveparty :!label _label
          (if (== _array_index (`KismetMathLibrary.RandomInteger` (`KismetArrayLibrary.Array_Length` _aliveparty)))
            (`KismetArrayLibrary.Array_Add` _targets _array_element)
            (break)))
        (else
          (bind _enemyparty (`/Game/Game/Blueprints/Pawns/BP_BattleManager.EnemyParty` _returnvalue))
          (for (_array_element_2 _array_index_2) _enemyparty :!label _label_2
            (if (== (`KismetMathLibrary.RandomInteger` (`KismetArrayLibrary.Array_Length` _enemyparty)) _array_index_2)
              (`KismetArrayLibrary.Array_Add` _targets _array_element_2)
              (break))))))
    (:`NewEnumerator2`
      (if _player
        (goto _label_2)
        (else
          (goto _label))))
    (:`NewEnumerator3`
      (if _player
        (`KismetArrayLibrary.Array_Append` _targets _aliveparty :!label _label_3)
        (else
          (`KismetArrayLibrary.Array_Append` _targets _enemyparty :!label _label_4))))
    (:`NewEnumerator6`
      (if _player
        (goto _label_4)
        (else
          (goto _label_3))))
    (:`NewEnumerator4`
      (`KismetArrayLibrary.Array_Append` _targets (`/Game/Game/Blueprints/Pawns/BP_BattleManager.AliveBattleChars` _returnvalue)))
    (:`NewEnumerator5`
      (`KismetArrayLibrary.Array_Add` _targets self))))

(fn `SetUp`
  (params (PlayerStruct :type "/Game/Game/Structs/S_Character Structure") (EnemyStruct :type "/Game/Game/Structs/S_Enemy Structure") (Player :type Boolean))
  (bind _output_get (set `self.Player` Player))
  (if _output_get
    (bind _output_get_2 (set `self.PStruct` PlayerStruct))
    (bind (_name _displayname _currentlvl _currentexp _class _icon _curstats _stats _levelupstats _equipment _allowedequipment _skills) (break `/Game/Game/Structs/S_Character` _output_get_2))
    (set `self.Stats` (make `/Game/Game/Structs/S_Stats` _name _displayname _currentlvl _icon _curstats _stats _equipment _skills))
    (else
      (bind _output_get_3 (set `self.EStruct` EnemyStruct))
      (bind (_name_2 _displayname_2 _lvl _icon_2 _expreward _goldreward _curstats_2 _stats_2 _loot _equipment_2 _skills_2) (break `/Game/Game/Structs/S_Enemy` _output_get_3))
      (set `self.Stats` (make `/Game/Game/Structs/S_Stats` _name_2 _displayname_2 _lvl _icon_2 _curstats_2 _stats_2 _equipment_2 _skills_2)))))

(fn `StartTurn`
  (`KismetArrayLibrary.Array_Clear` (`self.Targets`))
  (set `self.SkillToCast` (make `/Game/Game/Structs/Skills/S_Skill` "NewEnumerator0")))

(fn `TakeDamage`
  (params (dmg :type "Float (double-precision)"))
  (bind (_name _displayname _lvl _icon _curstats _stats) (break `/Game/Game/Structs/S_Stats` (`self.Stats`)))
  (bind _value (`BlueprintMapLibrary.Map_Find` _stats "NewEnumerator0"))
  (bind _returnvalue (- (`BlueprintMapLibrary.Map_Find` _curstats "NewEnumerator0") dmg))
  ; add branch for guarding
  (if (< _returnvalue 0.0)
    (`BlueprintMapLibrary.Map_Add` _curstats "NewEnumerator0")
    (elif (> _returnvalue _value)
      (`BlueprintMapLibrary.Map_Add` _curstats "NewEnumerator0" _value)
      (else
        (`BlueprintMapLibrary.Map_Add` _curstats "NewEnumerator0" _returnvalue))))
  (`self.AddRemoveChar`)
  (bind _returnvalue_2 (`GameplayStatics.GetActorOfClass` "/Game/Game/Blueprints/Pawns/BP_BattleManager.BP_BattleManager_C"))
  (`/Game/Game/Blueprints/Pawns/BP_BattleManager.Win/Lose` _returnvalue_2))

(fn `UserConstructionScript`)