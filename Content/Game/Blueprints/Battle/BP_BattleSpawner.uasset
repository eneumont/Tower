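; Battle spawn point that creates one player or enemy battler at its own transform when Spawn is called, chosen by the Player flag.
; Player battlers are set up from the GameInstance save's current party entry at Pos, while enemies receive only the flag.
; Each battler registers with BP_BattleManager's overall and side lists.
; Party members are sorted alive or dead by a current stat; enemies always start alive.
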(event `Spawn`
  (bind _returnvalue (`GameplayStatics.GetGameInstance`))
  (bind _player_ (`self.Player?`))
  (bind _returnvalue_2 (`self.GetTransform` self))
  (if _player_
    (bind _asbp_game_instance (cast `/Game/Game/Blueprints/Basics/BP_GameInstance` _returnvalue))
    (bind _returnvalue_3 (`|SpawnActorFromClass` "/Game/Game/Blueprints/Pawns/BP_BattlerP.BP_BattlerP_C" _returnvalue_2 "Undefined" "MultiplyWithRoot" null null))
    (`/Game/Game/Blueprints/Battle/BP_Battler.SetUp` :`self` _returnvalue_3 :`PlayerStruct` (`|GetArrayItem` (`.CurrentParty_14_F58803B34378013148F760BC06F2F439` (break `/Game/Game/Structs/S_SaveData` (`/Game/Game/Blueprints/Basics/BP_GameInstance.CurrentSaveData` _asbp_game_instance))) (`self.Pos`)) :`Player` _player_)
    (bind _returnvalue_4 (`GameplayStatics.GetActorOfClass` "/Game/Game/Blueprints/Pawns/BP_BattleManager.BP_BattleManager_C"))
    (`KismetArrayLibrary.Array_Add` (`/Game/Game/Blueprints/Pawns/BP_BattleManager.AllBattleChars` _returnvalue_4) _returnvalue_3)
    (`KismetArrayLibrary.Array_Add` (`/Game/Game/Blueprints/Pawns/BP_BattleManager.Party` _returnvalue_4) _returnvalue_3)
    (if (> (`BlueprintMapLibrary.Map_Find` (`.CurStats_82_32F2C6864CA14E01F5ED85B8E79787DE` (break `/Game/Game/Structs/S_Character` (`/Game/Game/Blueprints/Battle/BP_Battler.PStruct` _returnvalue_3))) "NewEnumerator0") 0.0)
      (`KismetArrayLibrary.Array_Add` (`/Game/Game/Blueprints/Pawns/BP_BattleManager.AliveBattleChars` _returnvalue_4) _returnvalue_3)
      (else
        (`KismetArrayLibrary.Array_Add` (`/Game/Game/Blueprints/Pawns/BP_BattleManager.DeadBattleChars` _returnvalue_4) _returnvalue_3)))
    (else
      (cast `/Game/Game/Blueprints/Basics/BP_GameInstance` _returnvalue)
      (bind _returnvalue_5 (`|SpawnActorFromClass` "/Game/Game/Blueprints/Enemies/BP_BattlerE.BP_BattlerE_C" _returnvalue_2 "Undefined" "MultiplyWithRoot" null null))
      (`/Game/Game/Blueprints/Battle/BP_Battler.SetUp` :`self` _returnvalue_5 :`Player` _player_)
      (bind _returnvalue_6 (`GameplayStatics.GetActorOfClass` "/Game/Game/Blueprints/Pawns/BP_BattleManager.BP_BattleManager_C"))
      (`KismetArrayLibrary.Array_Add` (`/Game/Game/Blueprints/Pawns/BP_BattleManager.AllBattleChars` _returnvalue_6) _returnvalue_5)
      (`KismetArrayLibrary.Array_Add` (`/Game/Game/Blueprints/Pawns/BP_BattleManager.EnemyParty` _returnvalue_6) _returnvalue_5)
      (`KismetArrayLibrary.Array_Add` (`/Game/Game/Blueprints/Pawns/BP_BattleManager.AliveBattleChars` _returnvalue_6) _returnvalue_5))))

(fn `UserConstructionScript`)