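; Base field spawner that spawns a configured actor class at its own transform or at a custom SpawnTransform, depending on DefaultSpawn.
; BeginPlay calls Spawn if none is active; Spawn sets SpawnActive and zeroes SpawnCountdown.
; While inactive with a non-negative SpawnTimer, Tick spawns again when countdown plus frame delta reaches the timer, without storing that sum.
; Nothing in this graph clears SpawnActive.
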(event `Spawn`
  (if (`self.DefaultSpawn`)
    (`|SpawnActorFromClass` (`self.SpawnActor`) (`self.GetTransform` self) "Undefined" "MultiplyWithRoot" null null)
    (else
      (`|SpawnActorFromClass` (`self.SpawnActor`) (`self.SpawnTransform`) "Undefined" "MultiplyWithRoot" null null)))
  (set `self.SpawnActive?` true)
  (set `self.SpawnCountdown` 0.0))

(event `self.ReceiveBeginPlay`
  (if (not (`self.SpawnActive?`))
    (`self.Spawn`)))

(event `self.ReceiveTick`
  (params (DeltaSeconds :type "Float (single-precision)"))
  (bind _spawntimer (`self.SpawnTimer`))
  (if (< _spawntimer 0.0)
    _
    (elif (`self.SpawnActive?`)
      _
      (elif (>= (+ (`self.SpawnCountdown`) DeltaSeconds) _spawntimer)
        (`self.Spawn`)))))

(fn `UserConstructionScript`)