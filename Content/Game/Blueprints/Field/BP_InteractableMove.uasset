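; BP_InteractableMove is a field map-transition actor that sends the player to another level.
; When a BP_FieldChar overlaps it, it runs its Interact event automatically.
; Interact passes MapSpawnPos to BP_GameInstance's NewMapSpawn, so the spawn point persists across the load, then opens the level named by MoveTo.
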(event `self.Interact`
  (bind _asbp_game_instance (cast `/Game/Game/Blueprints/Basics/BP_GameInstance` (`GameplayStatics.GetGameInstance`)))
  (`/Game/Game/Blueprints/Basics/BP_GameInstance.NewMapSpawn` _asbp_game_instance (`self.MapSpawnPos`))
  (`GameplayStatics.OpenLevel` (`KismetStringLibrary.Conv_StringToName` (`self.MoveTo`))))

(event `self.ReceiveActorBeginOverlap`
  (params (OtherActor :type "Actor Object Reference"))
  (cast `/Game/Game/Blueprints/Pawns/BP_FieldChar` OtherActor)
  (`self.Interact`))

(fn `UserConstructionScript`
  (`parent.UserConstructionScript`))