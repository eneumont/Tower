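; Player-side battler pawn for battles, extending a parent battler class.
; SetUp runs the parent setup, then passes the player struct's Class to the ABP_Player anim instance and sets its Battle flag.
; StartTurn and the construction script only forward to the parent.
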(fn `SetUp`
  (params (PlayerStruct :type "/Game/Game/Structs/S_Character Structure") (EnemyStruct :type "/Game/Game/Structs/S_Enemy Structure") (Player :type Boolean))
  (`parent.SetUp` PlayerStruct EnemyStruct Player)
  (bind _asabp_player (cast `/Game/Game/Animations/Player/ABP_Player` (`PaperZDAnimationComponent.AnimInstance` (`self.AnimationComponent`))))
  (set `/Game/Game/Animations/Player/ABP_Player.Class` (`.Class_77_9FFC13C443FC35F4C70B2EB3503483FC` (break `/Game/Game/Structs/S_Character` (`self.PStruct`))) _asabp_player)
  (set `/Game/Game/Animations/Player/ABP_Player.Battle` true _asabp_player))

(fn `StartTurn`
  (`parent.StartTurn`))

(fn `UserConstructionScript`
  (`parent.UserConstructionScript`))