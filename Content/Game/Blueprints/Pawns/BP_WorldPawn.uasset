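; BP_WorldPawn is a player pawn for world exploration, with movement and interaction through Enhanced Input.
; BeginPlay adds the IMCWorld mapping context, and Move applies input along fixed world axes while storing it as Directionality.
; Use runs a capsule overlap matching its own capsule and calls Interact on the first BP_InteractableBase found.
; The menu input calls a Menu event that is empty here.
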(event `EnhancedInput|/Game/Game/Inputs/Input-Actions/IA_Move`
  (params (ActionValue :type "Vector2D Structure") (ElapsedSeconds :type "Float (double-precision)") (TriggeredSeconds :type "Float (double-precision)") (InputAction :type "InputAction Object Reference" :default "/Game/Game/Inputs/Input-Actions/IA_Move.IA_Move"))
  (:`Triggered`
    (`self.AddMovementInput` (1.0 0.0 0.0) ActionValue_X)
    (`self.AddMovementInput` (0.0 -1.0 0.0) ActionValue_Y)
    (set `self.Directionality` (`KismetMathLibrary.MakeVector2D` ActionValue_X ActionValue_Y))))

(event `self.ReceiveBeginPlay`
  (bind _asplayer_controller (cast `PlayerController` (`self.GetController`)))
  (bind _returnvalue (pcsubsystem `EnhancedInputLocalPlayerSubsystem` _asplayer_controller))
  (`/Engine/EditorBlueprintResources/StandardMacros.IsValid` _returnvalue
    (:`Is Valid`
      (`EnhancedInputSubsystemInterface.AddMappingContext` _returnvalue "/Game/Game/Inputs/IMC/IMC-World.IMC-World" 0 (struct)))))

(event `EnhancedInput|/Game/Game/Inputs/Input-Actions/IA_Use`
  (params (ActionValue :type Boolean) (ElapsedSeconds :type "Float (double-precision)") (TriggeredSeconds :type "Float (double-precision)") (InputAction :type "InputAction Object Reference" :default "/Game/Game/Inputs/Input-Actions/IA_Use.IA_Use"))
  (bind _capsulecomponent (`self.CapsuleComponent`))
  (:`Triggered`
    (bind _outactors (`KismetSystemLibrary.CapsuleOverlapActors` (`SceneComponent.K2_GetComponentLocation` _capsulecomponent) (`CapsuleComponent.GetScaledCapsuleRadius` _capsulecomponent) (`CapsuleComponent.CapsuleHalfHeight` _capsulecomponent) (`|MakeArray` "ObjectTypeQuery1" :!type "EObjectTypeQuery Enum") "/Game/Game/Blueprints/Interactables/BP_InteractableBase.BP_InteractableBase_C"))
    (bind _asbp_interactable_base (cast `/Game/Game/Blueprints/Interactables/BP_InteractableBase` (`|GetArrayItem` _outactors)))
    (`/Game/Game/Blueprints/Interactables/BP_InteractableBase.Interact` _asbp_interactable_base)))

(event `EnhancedInput|/Game/Game/Inputs/Input-Actions/IA_Menu`
  (params (ActionValue :type Boolean) (ElapsedSeconds :type "Float (double-precision)") (TriggeredSeconds :type "Float (double-precision)") (InputAction :type "InputAction Object Reference" :default "/Game/Game/Inputs/Input-Actions/IA_Menu.IA_Menu"))
  (:`Triggered`
    (`self.Menu`)))

(event `Menu`)

(fn `UserConstructionScript`)