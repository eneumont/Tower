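; BP_FieldChar is the player-controlled field character, shown as a flipbook sprite of the first party member's class.
; On BeginPlay it adds the field Enhanced Input context and picks the idle flipbook from the game instance's save data.
; Move input drives world-axis movement and stores Directionality, while Use calls Interact on the first interactable overlapping the capsule.
; Menu and Attack are empty stubs.
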(event `EnhancedInput|/Game/Game/Inputs/Input-Actions/IA_Move`
  (params (ActionValue :type "Vector2D Structure") (ElapsedSeconds :type "Float (double-precision)") (TriggeredSeconds :type "Float (double-precision)") (InputAction :type "InputAction Object Reference" :default "/Game/Game/Inputs/Input-Actions/IA_Move.IA_Move"))
  (:`Triggered`
    (`self.AddMovementInput` (1.0 0.0 0.0) ActionValue_X)
    (`self.AddMovementInput` (0.0 -1.0 0.0) ActionValue_Y)
    (set `self.Directionality` (`KismetMathLibrary.MakeVector2D` ActionValue_X ActionValue_Y))))

(event `self.ReceiveBeginPlay`
  (bind _asplayer_controller (cast `PlayerController` (`self.GetController`)))
  (bind _returnvalue (pcsubsystem `EnhancedInputLocalPlayerSubsystem` _asplayer_controller))
  (`/Engine/EditorBlueprintResources/StandardMacros.IsValid` _returnvalue
    (:`Is Valid`
      (`EnhancedInputSubsystemInterface.AddMappingContext` _returnvalue "/Game/Game/Inputs/IMC/IMC-Field.IMC-Field" 0 (struct))
      (`self.ChangeFielder`))))

(event `EnhancedInput|/Game/Game/Inputs/Input-Actions/IA_Use`
  (params (ActionValue :type Boolean) (ElapsedSeconds :type "Float (double-precision)") (TriggeredSeconds :type "Float (double-precision)") (InputAction :type "InputAction Object Reference" :default "/Game/Game/Inputs/Input-Actions/IA_Use.IA_Use"))
  (bind _capsulecomponent (`self.CapsuleComponent`))
  (:`Triggered`
    (bind _outactors (`KismetSystemLibrary.CapsuleOverlapActors` (`SceneComponent.K2_GetComponentLocation` _capsulecomponent) (`CapsuleComponent.CapsuleRadius` _capsulecomponent) (`CapsuleComponent.CapsuleHalfHeight` _capsulecomponent) (`|MakeArray` "ObjectTypeQuery2" :!type "EObjectTypeQuery Enum") "/Game/Game/Blueprints/Interactables/BP_InteractableBase.BP_InteractableBase_C"))
    (bind _asbp_interactable_base (cast `/Game/Game/Blueprints/Interactables/BP_InteractableBase` (`|GetArrayItem` _outactors)))
    (`/Game/Game/Blueprints/Interactables/BP_InteractableBase.Interact` _asbp_interactable_base)))

(event `EnhancedInput|/Game/Game/Inputs/Input-Actions/IA_Menu`
  (params (ActionValue :type Boolean) (ElapsedSeconds :type "Float (double-precision)") (TriggeredSeconds :type "Float (double-precision)") (InputAction :type "InputAction Object Reference" :default "/Game/Game/Inputs/Input-Actions/IA_Menu.IA_Menu"))
  (:`Triggered`
    (`self.Menu`)))

(event `ChangeFielder`
  (bind _sprite (`self.Sprite`))
  (bind _asbp_game_instance (cast `/Game/Game/Blueprints/Basics/BP_GameInstance` (`GameplayStatics.GetGameInstance`)))
  (switch `/Game/Game/Enums/E_Class` (`.Class_77_9FFC13C443FC35F4C70B2EB3503483FC` (break `/Game/Game/Structs/S_Character` (`|GetArrayItem` (`.CurrentParty_14_F58803B34378013148F760BC06F2F439` (break `/Game/Game/Structs/S_SaveData` (`/Game/Game/Blueprints/Basics/BP_GameInstance.CurrentSaveData` _asbp_game_instance))))))
    (:`NewEnumerator1`
      (`PaperFlipbookComponent.SetFlipbook` _sprite "/Game/Game/Images/Sprites/Knight/Field/Down/knight_field_idle.knight_field_idle"))
    (:`NewEnumerator2`
      (`PaperFlipbookComponent.SetFlipbook` _sprite "/Game/Game/Images/Sprites/Thief/Field/Down/thief_field_idle.thief_field_idle"))
    (:`NewEnumerator3`
      (`PaperFlipbookComponent.SetFlipbook` _sprite "/Game/Game/Images/Sprites/Mage/Field/Down/mage_field_idle.mage_field_idle"))
    (:`NewEnumerator4`
      (`PaperFlipbookComponent.SetFlipbook` _sprite "/Game/Game/Images/Sprites/Cleric/Field/Down/cleric_field_idle.cleric_field_idle"))))

(event `Menu`)

(event `EnhancedInput|/Game/Game/Inputs/Input-Actions/IA_Attack`
  (params (ActionValue :type Boolean) (ElapsedSeconds :type "Float (double-precision)") (TriggeredSeconds :type "Float (double-precision)") (InputAction :type "InputAction Object Reference" :default "/Game/Game/Inputs/Input-Actions/IA_Attack.IA_Attack")))

(fn `UserConstructionScript`)