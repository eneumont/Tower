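; BP_BattleManager sets up a battle and resolves its outcome.
; On BeginPlay it calls Spawn on every BP_BattleSpawner, then has the first top-level WBP_Battle widget create the turn order.
; WinLose checks the party arrays: victory opens the map named in the game instance's current save data, while a party wipe opens WorldMap.
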(event `self.ReceiveBeginPlay`
  (bind _outactors (`GameplayStatics.GetAllActorsOfClass` "/Game/Game/Blueprints/Battle/BP_BattleSpawner.BP_BattleSpawner_C"))
  (for _array_element _outactors
    (`/Game/Game/Blueprints/Battle/BP_BattleSpawner.Spawn` _array_element))
  (bind _foundwidgets (`WidgetBlueprintLibrary.GetAllWidgetsOfClass` "/Game/Game/UI/Battle/WBP_Battle.WBP_Battle_C"))
  (`/Game/Game/UI/Battle/WBP_Battle.CreateTurnOrder` (`|GetArrayItem` _foundwidgets)))

(fn `UserConstructionScript`)

(fn `Win/Lose`
  (if (> (`KismetArrayLibrary.Array_Length` (`self.AliveParty`)) 0)
    (if (not (> (`KismetArrayLibrary.Array_Length` (`self.EnemyParty`)) 0))
      (bind _asbp_game_instance (cast `/Game/Game/Blueprints/Basics/BP_GameInstance` (`GameplayStatics.GetGameInstance`)))
      (`GameplayStatics.OpenLevel` (`KismetStringLibrary.Conv_StringToName` (`.MapName_37_490558294894E216AB5D20BDAC0F04C5` (break `/Game/Game/Structs/S_SaveData` (`/Game/Game/Blueprints/Basics/BP_GameInstance.CurrentSaveData` _asbp_game_instance))))))
    (else
      (`GameplayStatics.OpenLevel` "WorldMap"))))