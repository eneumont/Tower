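; BP_FieldFoe is a field enemy Blueprint with a CharacterMovement component and a helper for changing its speed.
; UpdateWalkSpeed sets the component's MaxWalkSpeed to the value passed in.
; Begin and end overlap events filter for BP_FieldChar and cast to BP_GameInstance, but take no further action.
; Save data and inventory lookups on the game instance are present but unused, and the construction script is empty.
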(event `self.ReceiveActorBeginOverlap`
  (params (OtherActor :type "Actor Object Reference"))
  (cast `/Game/Game/Blueprints/Pawns/BP_FieldChar` OtherActor)
  (bind _asbp_game_instance (cast `/Game/Game/Blueprints/Basics/BP_GameInstance` (`GameplayStatics.GetGameInstance`))))

(event `self.ReceiveActorEndOverlap`
  (params (OtherActor :type "Actor Object Reference"))
  (cast `/Game/Game/Blueprints/Pawns/BP_FieldChar` OtherActor)
  (bind _asbp_game_instance (cast `/Game/Game/Blueprints/Basics/BP_GameInstance` (`GameplayStatics.GetGameInstance`))))

(fn `Update Walk Speed`
  (params (NewWalkSpeed :type "Float (double-precision)"))
  (set `CharacterMovementComponent.MaxWalkSpeed` NewWalkSpeed (`self.CharacterMovement`)))

(fn `UserConstructionScript`)