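; BP_BattlerE is an enemy battler Blueprint that takes its turn by using random skills from its Stats.
; StartTurn runs the parent logic, then, while Done is true, calls SetTargets and CastSkill in a loop.
; Each call draws its own random index into Stats.Skills, so the skill used for targeting can differ from the one cast.
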(fn `StartTurn`
  (bind (_name _displayname _lvl _icon _curstats _stats _equipment _skills) (break `/Game/Game/Structs/S_Stats` (`self.Stats`)))
  (bind _output (`|GetArrayItem` _skills (`KismetMathLibrary.RandomInteger` (`KismetArrayLibrary.Array_Length` _skills))))
  (`parent.StartTurn`)
  (while (`self.Done`)
    (`self.SetTargets` _output)
    (`self.CastSkill` _output)))

(fn `UserConstructionScript`
  (`parent.UserConstructionScript`))