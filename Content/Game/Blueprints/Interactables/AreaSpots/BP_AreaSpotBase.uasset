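; Base interactable area spot that opens a level by its map name when the player interacts with it.
; On BeginPlay it fills its WBP_AreaSpot widget with the map's description, picture and name, trimming five characters from the end of the name for display.
; The widget component shows while a BP_WorldChar overlaps the actor and hides when the overlap ends.
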(event `self.ReceiveBeginPlay`
  (bind _aswbp_area_spot (cast `/Game/Game/UI/World/WBP_AreaSpot` (`WidgetComponent.GetWidget` (`self.Widget`))))
  (set `/Game/Game/UI/World/WBP_AreaSpot.Name` (`KismetStringLibrary.LeftChop` (`self.MapName`) 5) _aswbp_area_spot)
  (set `/Game/Game/UI/World/WBP_AreaSpot.Description` (`self.MapDescription`) _aswbp_area_spot)
  (set `/Game/Game/UI/World/WBP_AreaSpot.Pic` (`self.MapPic`) _aswbp_area_spot))

(event `self.Interact`
  (`GameplayStatics.OpenLevel` (`KismetStringLibrary.Conv_StringToName` (`self.MapName`))))

(event `self.ReceiveActorBeginOverlap`
  (params (OtherActor :type "Actor Object Reference"))
  (cast `/Game/Game/Blueprints/Pawns/BP_WorldChar` OtherActor)
  (`SceneComponent.SetVisibility` (`self.Widget`) true false))

(event `self.ReceiveActorEndOverlap`
  (params (OtherActor :type "Actor Object Reference"))
  (cast `/Game/Game/Blueprints/Pawns/BP_WorldChar` OtherActor)
  (`SceneComponent.SetVisibility` (`self.Widget`) false false))

(fn `UserConstructionScript`
  (`parent.UserConstructionScript`))