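; BP_InteractableChest is an interactable chest Blueprint tied to an item entry in the DT_FoundItems data table.
; On BeginPlay and on Interact, it looks up the row named by ItemName and tests whether its Amount is zero.
; Both checks lead to no action, and the construction script only calls its parent.
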(event `self.ReceiveBeginPlay`
  (bind _returnvalue (`|GetDataTableRow` "/Game/Game/Datatables/DT_FoundItems.DT_FoundItems" (`KismetStringLibrary.Conv_StringToName` (`self.ItemName`)))
    (:`then`
      (if (== (`.Amount_5_DC1C01BA423CF1CA625959947FBFE884` (break `/Game/Game/Structs/S_ItemDynamicData` _returnvalue)) 0)
        _))))

(event `self.Interact`
  (bind _returnvalue (`|GetDataTableRow` "/Game/Game/Datatables/DT_FoundItems.DT_FoundItems" (`KismetStringLibrary.Conv_StringToName` (`self.ItemName`)))
    (:`then`
      (if (== (`.Amount_5_DC1C01BA423CF1CA625959947FBFE884` (break `/Game/Game/Structs/S_ItemDynamicData` _returnvalue)) 0)
        _))))

(fn `UserConstructionScript`
  (`parent.UserConstructionScript`))