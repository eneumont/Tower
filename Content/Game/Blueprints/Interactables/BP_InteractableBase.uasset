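; BP_InteractableBase is a base actor for interactable items that removes itself from the level based on the DT_FoundItems data table.
; On BeginPlay it looks up the row named by ItemName and destroys itself if that row's Amount is non-zero.
; On Interact it repeats the lookup and destroys itself if Amount is zero.
; It only reads the table, and does nothing when no row matches.
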(event `self.ReceiveBeginPlay`
  (bind _returnvalue (`|GetDataTableRow` "/Game/Game/Datatables/DT_FoundItems.DT_FoundItems" (`KismetStringLibrary.Conv_StringToName` (`self.ItemName`)))
    (:`then`
      (if (not (== (`.Amount_5_DC1C01BA423CF1CA625959947FBFE884` (break `/Game/Game/Structs/S_ItemDynamicData` _returnvalue)) 0))
        (`self.K2_DestroyActor`)))))

(event `Interact`
  (bind _returnvalue (`|GetDataTableRow` "/Game/Game/Datatables/DT_FoundItems.DT_FoundItems" (`KismetStringLibrary.Conv_StringToName` (`self.ItemName`)))
    (:`then`
      (if (== (`.Amount_5_DC1C01BA423CF1CA625959947FBFE884` (break `/Game/Game/Structs/S_ItemDynamicData` _returnvalue)) 0)
        (`self.K2_DestroyActor`)))))

(fn `UserConstructionScript`)